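; Pressure plate actor that sinks its mesh when a cast-filtered actor overlaps it and returns it three seconds after that overlap ends.
; Both overlap events search all Door actors for a DoorID matching PressurePlateID.
; A match only sets the Door variable to None, and the following validity check leads to no action, so the plate drives no door as written.
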(event EventBeginPlay)

(event EventTick
  (params (DeltaSeconds :type Float%20%28single-precision%29)))

(event Collision|EventActorBeginOverlap
  (params (OtherActor :type Actor%20Object%20Reference))
  (Utilities|Casting|CastTo OtherActor)
  (Components|MoveComponentTo (Variables|Default|GetStaticMesh) "0, 0,-10.000000" "0, 0, 0" false false 0.5 false)
  (bind _outactors (Actor|GetAllActorsOfClass "/Game/UnusedAndStarter/Buttons/PressureDoor/Door.Door_C"))
  (for _array_element _outactors
    (if (== (Variables|Default|GetDoorID _array_element) (Variables|Default|GetPressurePlateID))
      (Variables|Default|SetDoor 0)))
  (Utilities|IsValid (Variables|Default|GetDoor)))

(event Collision|EventActorEndOverlap
  (params (OtherActor :type Actor%20Object%20Reference))
  (Utilities|Casting|CastTo OtherActor)
  (Utilities|FlowControl|Delay 3.0)
  (Components|MoveComponentTo (Variables|Default|GetStaticMesh) "0, 0, 0" "0, 0, 0" false false 0.2 false)
  (bind _outactors (Actor|GetAllActorsOfClass "/Game/UnusedAndStarter/Buttons/PressureDoor/Door.Door_C"))
  (for _array_element _outactors
    (if (== (Variables|Default|GetDoorID _array_element) (Variables|Default|GetPressurePlateID))
      (Variables|Default|SetDoor 0)))
  (Utilities|IsValid (Variables|Default|GetDoor)))

(fn ConstructionScript)